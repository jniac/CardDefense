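; Card manager component that detects which card actor is under the player's mouse cursor.
; Each tick, GetTraceCard line traces from the pawn's camera along the deprojected cursor direction on a dedicated trace channel and casts the hit to a generic card.
; When the hovered card changes, the previous card receives HoverExit and the new one HoverEnter.
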(event `self.ReceiveTick`
  (params (DeltaSeconds :type "Float (single-precision)"))
  (bind _returnvalue (`GameplayStatics.GetPlayerController` 0))
  (bind (_locationx _locationy) (`PlayerController.GetMousePosition` _returnvalue))
  (bind (_hit _outhit _card) (`self.GetTraceCard` _returnvalue _locationx _locationy))
  (if (!= _card (`self.hover`))
    (set `self.hoverOld` (`self.hover`))
    (set `self.hover` _card)
    ; Hover Enter/Exit
    (`/Engine/EditorBlueprintResources/StandardMacros.IsValid` (`self.hoverOld`)
      (:`Is Valid`
        (`/Game/Art/jnc/Blueprints/jnc_BP_GenericCard.HoverExit` (`self.hoverOld`)))
      (:`Is Not Valid`
        _))
    (`/Engine/EditorBlueprintResources/StandardMacros.IsValid` (`self.hover`)
      (:`Is Valid`
        (`/Game/Art/jnc/Blueprints/jnc_BP_GenericCard.HoverEnter` (`self.hover`)))
      (:`Is Not Valid`))))

(fn `GetTraceCard`
  (params (Player :type "PlayerController Object Reference") (ScreenPosition_X :type "Float (double-precision)") (ScreenPosition_Y :type "Float (double-precision)"))
  (returns (hit :type Boolean) (outHit :type "HitResult Structure") (card :type "/Game/Art/jnc/Blueprints/jnc_BP_GenericCard Object Reference"))
  (bind _returnvalue (`SceneComponent.K2_GetComponentLocation` (`/Game/Art/jnc/Blueprints/jnc_BP_CardDefensePawn.Camera` (`/Game/Art/jnc/Blueprints/jnc_BPL_CardDefenseUtils.CD_PlayerPawn`))))
  (bind (_outhit _returnvalue_2) (`KismetSystemLibrary.LineTraceSingle` _returnvalue (+ _returnvalue (* (`.WorldDirection` (`GameplayStatics.DeprojectScreenToWorld` Player (`KismetMathLibrary.MakeVector2D` ScreenPosition_X ScreenPosition_Y))) 100000.0)) "TraceTypeQuery3"))
  (if _returnvalue_2
    _
    (else
      _))
  (bind _asjnc_bp_generic_card (cast `/Game/Art/jnc/Blueprints/jnc_BP_GenericCard` (`.HitActor` (`GameplayStatics.BreakHitResult` _outhit)))
    (:`then`
      _)
    (:`CastFailed`
      _))
  (return _returnvalue_2 _outhit _asjnc_bp_generic_card))