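; Actor Blueprint that lays out a fanned hand of generic card actors along a circular arc.
; The construction script clears previous cards, then spawns one child actor component per card and caches components and cast card actors.
; Arc length per gap over radius sets the centred angular spread; each card rolls to follow the curve, offset down by the radius and composed with the actor transform.
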(fn `CreateCards`
  (locals (indexMax :type Integer) (t :type "Float (double-precision)") (angleDelta :type "Float (double-precision)"))
  (bind _returnvalue (`KismetMathLibrary.RadiansToDegrees` (`KismetMathLibrary.Lerp` (* (`local.angleDelta`) -0.5) (* (`local.angleDelta`) 0.5) (`local.t`))))
  (bind (_point_x _point_y _point_z) (`KismetMathLibrary.BreakVector` (`/Game/Library/jnc_BP_BasicUtils.OnCircle` (+ _returnvalue 90.0) (`self.radius`) "NewEnumerator1")))
  (`self.DestroyAllCards`)
  (set `local.indexMax` (- (`self.cardCount`) 1))
  (set `local.angleDelta` (/ (* (`self.arc`) (`local.indexMax`)) (`self.radius`)))
  (for _index (range (+ (`local.indexMax`) 1))
    ; T
    (set `local.t` (/ (`KismetMathLibrary.Conv_IntToDouble` _index) (`KismetMathLibrary.Conv_IntToDouble` (`local.indexMax`))))
    (bind _returnvalue_2 (`AddComponent|NODE_AddChildActorComponent-0`))
    (`KismetArrayLibrary.Array_Add` (`self.cardComponents`) _returnvalue_2)
    (`ChildActorComponent.SetChildActorClass` _returnvalue_2 "/Game/Art/jnc/Blueprints/jnc_BP_GenericCard.jnc_BP_GenericCard_C")
    (bind _childactor (`ChildActorComponent.ChildActor` _returnvalue_2))
    (`self.K2_SetActorTransform` _childactor (`KismetMathLibrary.ComposeTransforms` (`KismetMathLibrary.MakeTransform` (`KismetMathLibrary.MakeVector` 0.0 _point_y (- _point_z (`self.radius`))) (`KismetMathLibrary.MakeRotator` (+ (.roll (`self.cardRotation`)) (* _returnvalue -1.0)) (.pitch (`self.cardRotation`)) (.yaw (`self.cardRotation`)))) (`self.GetTransform`)) false false)
    (bind _asjnc_bp_generic_card (cast `/Game/Art/jnc/Blueprints/jnc_BP_GenericCard` _childactor)
      (:`then`
        (`KismetArrayLibrary.Array_Add` (`self.cardActors`) _asjnc_bp_generic_card))
      (:`CastFailed`
        (`KismetSystemLibrary.PrintString` "Oops")))))

(fn `DestroyAllCards`
  (for _array_element (`self.cardComponents`)
    (`ActorComponent.K2_DestroyComponent` _array_element))
  (`KismetArrayLibrary.Array_Clear` (`self.cardComponents`))
  (`KismetArrayLibrary.Array_Clear` (`self.cardActors`)))

(fn `UserConstructionScript`
  (`self.CreateCards`))