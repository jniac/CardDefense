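; Generic card actor that displays a UMG widget through its CardWidget component, apparently for a card defense game.
; InitWidget creates the widget and assigns it to the component, while hover enter and exit events forward to it through the card interface.
; LineTraceCard tests CardHitArea against a mouse ray from the defense pawn's camera.
; Its only use, a hover scale-up of the root, is disconnected and never runs.
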(event `self.ReceiveBeginPlay`)

(event `self.ReceiveTick`
  (params (DeltaSeconds :type "Float (single-precision)")))

(event `HoverEnter`
  (bind _asjnc_bpi_card (cast `/Game/Art/jnc/Blueprints/jnc_BPI_Card` (`WidgetComponent.GetWidget` (`self.CardWidget`))))
  (`/Game/Art/jnc/Blueprints/jnc_BPI_Card.HoverEnter` _asjnc_bpi_card))

(event `HoverExit`
  (bind _asjnc_bpi_card (cast `/Game/Art/jnc/Blueprints/jnc_BPI_Card` (`WidgetComponent.GetWidget` (`self.CardWidget`))))
  (`/Game/Art/jnc/Blueprints/jnc_BPI_Card.HoverExit` _asjnc_bpi_card))

(fn `InitWidget`
  (bind _asuser_widget (castclass `UserWidget` null))
  (bind _returnvalue (`|CreateWidget` _asuser_widget))
  (`WidgetComponent.SetWidget` (`self.CardWidget`) _returnvalue))

(fn `LineTraceCard`
  (returns (ReturnValue :type Boolean))
  (bind _returnvalue (`GameplayStatics.GetPlayerController` 0))
  (bind (_locationx _locationy) (`PlayerController.GetMousePosition` _returnvalue))
  (bind _asjnc_bp_card_defense_pawn (cast `/Game/Art/jnc/Blueprints/jnc_BP_CardDefensePawn` (`GameplayStatics.GetPlayerPawn` 0)))
  (bind _returnvalue_2 (`SceneComponent.K2_GetComponentLocation` (`/Game/Art/jnc/Blueprints/jnc_BP_CardDefensePawn.Camera` _asjnc_bp_card_defense_pawn)))
  (bind (_hitlocation _hitnormal _bonename _outhit _returnvalue_3) (`PrimitiveComponent.K2_LineTraceComponent` (`self.CardHitArea`) _returnvalue_2 (+ _returnvalue_2 (* (`.WorldDirection` (`GameplayStatics.DeprojectScreenToWorld` _returnvalue (`KismetMathLibrary.MakeVector2D` _locationx _locationy))) 100000.0)) true false false))
  (return _returnvalue_3))

(fn `UserConstructionScript`)